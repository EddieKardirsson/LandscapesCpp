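; Voxel terrain actor that builds a blocky heightmap from instanced static meshes in its construction script.
; A nested loop over VoxelSize samples 2D simplex noise at grid coordinates from ActorLocation, which involves the actor's world position and VoxelDensity.
; AddNoise scales and floors each noise value into stepped heights, adding one mesh instance per column on a 100-unit grid.
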(event EventBeginPlay)

(event Collision|EventActorBeginOverlap
  (params (OtherActor :type Actor%20Object%20Reference)))

(event EventTick
  (params (DeltaSeconds :type Float%20%28single-precision%29)))

(fn ConstructionScript
  (bind _voxelsize (Variables|Default|GetVoxelSize))
  (for _index (range 0 _voxelsize)
    (for _index_2 (range 0 _voxelsize)
      (bind _returnvalue (Class|SimplexNoiseBPLibrary|SimplexNoise2D (.X (Utilities|ActorLocation _index _index_2)) (.Y (Utilities|ActorLocation _index _index_2)) 1.0))
      (CallFunction|AddNoise _returnvalue (* _index 1e+02) (* _index_2 1e+02)))))

(fn AddNoise
  (params (Noise :type Float%20%28single-precision%29) (XTransform :type Float%20%28single-precision%29) (YTransform :type Float%20%28single-precision%29))
  (Components|InstancedStaticMesh|AddInstance (Variables|Default|GetInstancedStaticMesh) (Math|Conversions|ToTransform(Vector) (Math|Vector|MakeVector XTransform YTransform (* (Math|Float|Floor (* 10 Noise)) 1e+02)))))